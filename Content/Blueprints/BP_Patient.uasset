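; BP_Patient is a patient that is revived by receiving a number of CPR actions.
; BeginPlay rolls a small random count of required CPRs.
; GetCPR decrements that count and prints a revival message once it reaches zero or below.
; A DoOnce gate limits CPR to one count per second, reopened by ResetCPR after a delay.
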(event Custom|Reset%20CPR
  (Utilities|FlowControl|DoOnce false) ; enters at Reset
)

(event EventBeginPlay
  ;[1 1 1] Number Of CPR Required To Patient
  (Variables|Default|SetCPR_Required_To_Save (Math|Random|RandomIntegerinRange 3 5)))

(event Collision|EventActorBeginOverlap
  (params (OtherActor :type Actor%20Object%20Reference)))

(event EventTick
  (params (DeltaSeconds :type Float%20%28single-precision%29)))

(event EventGetCPR
  (Utilities|FlowControl|DoOnce false
    (:Completed
      (Variables|Default|SetCPR_Required_To_Save (- (Variables|Default|GetCPR_Required_To_Save) 1))
      (if (<= (Variables|Default|GetCPR_Required_To_Save) 0)
        (Development|PrintString "Patient Revived" true true "(R=0.000000,G=0.660000,B=1.000000,A=1.000000)" 2.0 "a"))
      (Utilities|FlowControl|Delay 1.0)
      (CallFunction|ResetCPR))))

(fn ConstructionScript)